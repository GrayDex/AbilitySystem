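; Player character Blueprint that feeds health, mana and strength changes to the player's on-screen HUD.
; BeginPlay casts the controller to BP_PlayerController and caches the reference.
; Each stat-change event divides the current value by its maximum and calls SetPercentage on the matching WBP_GlassBall in the controller's PrimaryUI, so the HUD updates on events without using Tick.
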(event `self.ReceiveBeginPlay`
  (`parent.ReceiveBeginPlay`)
  ;[1 1 1] Set PlayerControllerRef
  (bind _asbp_player_controller (cast `/Game/Blueprints/BP_PlayerController` (`self.GetController`)))
  (set `self.PlayerControllerRef` _asbp_player_controller))

(event `self.BP_OnHealthChanged`
  (params (Health :type "Float (single-precision)") (MaxHealth :type "Float (single-precision)"))
  ;[1 1 1] Update character state values in instances WBP_GlassBall setted in Primary ui. call event SetPercentage, that init in WBP_GlassBall
  (`/Game/Blueprints/UI/Player_PrimaryUI/GlassBallComponent/WBP_GlassBall.SetPercentage` (`/Game/Blueprints/UI/Player_PrimaryUI/WBP_PrimaryUI.Health_GlassBall` (`/Game/Blueprints/BP_PlayerController.PrimaryUI` (`self.PlayerControllerRef`))) (/ Health MaxHealth)))

(event `self.BP_OnManaChanged`
  (params (Mana :type "Float (single-precision)") (MaxMana :type "Float (single-precision)"))
  ;[1 1 1] Update character state values in instances WBP_GlassBall setted in Primary ui. call event SetPercentage, that init in WBP_GlassBall
  (`/Game/Blueprints/UI/Player_PrimaryUI/GlassBallComponent/WBP_GlassBall.SetPercentage` (`/Game/Blueprints/UI/Player_PrimaryUI/WBP_PrimaryUI.Mana_GlassBall` (`/Game/Blueprints/BP_PlayerController.PrimaryUI` (`self.PlayerControllerRef`))) (/ Mana MaxMana)))

(event `self.BP_OnStrenghtChanged`
  (params (Strenght :type "Float (single-precision)") (MaxStrenght :type "Float (single-precision)"))
  ;[1 1 1] Update character state values in instances WBP_GlassBall setted in Primary ui. call event SetPercentage, that init in WBP_GlassBall
  (`/Game/Blueprints/UI/Player_PrimaryUI/GlassBallComponent/WBP_GlassBall.SetPercentage` (`/Game/Blueprints/UI/Player_PrimaryUI/WBP_PrimaryUI.Strenght_GlassBall` (`/Game/Blueprints/BP_PlayerController.PrimaryUI` (`self.PlayerControllerRef`))) (/ Strenght MaxStrenght)))

(fn `UserConstructionScript`
  (`parent.UserConstructionScript`))