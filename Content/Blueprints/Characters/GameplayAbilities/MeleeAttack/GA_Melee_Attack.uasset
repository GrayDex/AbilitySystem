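; GA_Melee_Attack is a Gameplay Ability that performs a melee attack by playing a Shinby attack montage.
; It commits the ability, plays the montage, and waits for the Skill.melee.dealDamage gameplay event to apply the melee damage effect to the event's target.
; The ability ends when the montage completes, blends out, or is interrupted or cancelled, with debug prints for instigator, target and ability end.
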(event `self.K2_ActivateAbility`
  ;[1 1 1] need calls for test cooldown ended setted in this in gameplayeffects
  (`self.K2_CommitAbility`)
  (`AbilityTask_PlayMontageAndWait.CreatePlayMontageAndWaitProxy` "None" "/Game/Blueprints/Characters/Animations/AM_Shinby_MileeAtk.AM_Shinby_MileeAtk"
    (:`then`
      (bind (_asynctaskproxy _payload) (`AbilityTask_WaitGameplayEvent.WaitGameplayEvent` (struct :`TagName` "skill.melee.dealDamage") null)
        (:`EventReceived`
          (bind (_eventtag _instigator _target) (break `GameplayEventData` _payload))
          (`self.Print` _instigator _target)
          (`self.BP_ApplyGameplayEffectToTarget` (`AbilitySystemBlueprintLibrary.AbilityTargetDataFromActor` _target) "/Game/Blueprints/Characters/GameplayAbilities/MeleeAttack/GE_Apply_Melee_Damage.GE_Apply_Melee_Damage_C"))))
    (:`OnCompleted`
      ;[1 1 1] Begin event OnEndAbility
      (`self.K2_EndAbility` :!label _label))
    (:`OnBlendOut`
      (goto _label))
    (:`OnInterrupted`
      (goto _label))
    (:`OnCancelled`
      (goto _label))))

(event `self.K2_OnEndAbility`
  (params (bWasCancelled :type Boolean))
  (`KismetSystemLibrary.PrintString` (`KismetStringLibrary.Concat_StrStr` "Ability: " (`KismetSystemLibrary.GetObjectName` self) " end.")))

(fn `Print`
  (params (Instigator :type "Object Object Reference") (Target :type "Actor Object Reference"))
  (`KismetSystemLibrary.PrintString` (`KismetStringLibrary.Concat_StrStr` "Instigator: " (`KismetSystemLibrary.GetDisplayName` Instigator)))
  (`KismetSystemLibrary.PrintString` (`KismetStringLibrary.Concat_StrStr` "Target: " (`KismetSystemLibrary.GetDisplayName` Target))))