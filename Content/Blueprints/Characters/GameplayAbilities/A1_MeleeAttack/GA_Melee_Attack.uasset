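; Gameplay ability for a melee attack that plays the Shinbi attack montage and damages the target it hits.
; On activation it commits the ability, plays the montage and waits for a Skill.melee.dealDamage gameplay event.
; The event payload supplies the target, which receives the melee damage gameplay effect.
; The ability ends when the montage completes, blends out, is interrupted or cancelled, with debug prints along the way.
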(event `self.K2_ActivateAbility`
  ;[1 1 1] need calls for test cooldown ended setted in this in gameplayeffects
  (`self.K2_CommitAbility`)
  (`AbilityTask_PlayMontageAndWait.CreatePlayMontageAndWaitProxy` "None" "/Game/Blueprints/Characters/Animations/AM_MeleeAttack_Shinbi.AM_MeleeAttack_Shinbi" 1.0 "None"
    (:`then`
      ;[1 1 1] wait event with any tag to continue execution. in event will be set target, that be set to apply damage in here
      (bind (_asynctaskproxy _payload) (`AbilityTask_WaitGameplayEvent.WaitGameplayEvent` (struct :`TagName` "skill.melee.dealDamage") null)
        (:`EventReceived`
          (bind (_eventtag _instigator _target) (break `GameplayEventData` _payload))
          (`self.Print` _instigator _target)
          ;[1 1 1] Call GE_AttackDamage for apply damage to target
          (`self.BP_ApplyGameplayEffectToTarget` (`AbilitySystemBlueprintLibrary.AbilityTargetDataFromActor` _target) "/Game/Blueprints/Characters/GameplayAbilities/A1_MeleeAttack/GE_Apply_Melee_Damage.GE_Apply_Melee_Damage_C"))))
    (:`OnCompleted`
      ;[1 1 1] Call event OnEndAbility
      (`self.K2_EndAbility` :!label _label))
    (:`OnBlendOut`
      (goto _label))
    (:`OnInterrupted`
      (goto _label))
    (:`OnCancelled`
      (goto _label))))

(event `self.K2_OnEndAbility`
  (params (bWasCancelled :type Boolean))
  (`KismetSystemLibrary.PrintString` (`KismetStringLibrary.Concat_StrStr` "Ability: " (`KismetSystemLibrary.GetObjectName` self) " end.")))

(fn `Print`
  (params (Instigator :type "Object Object Reference") (Target :type "Actor Object Reference"))
  (`KismetSystemLibrary.PrintString` (`KismetStringLibrary.Concat_StrStr` "Instigator: " (`KismetSystemLibrary.GetDisplayName` Instigator)))
  (`KismetSystemLibrary.PrintString` (`KismetStringLibrary.Concat_StrStr` "Target: " (`KismetSystemLibrary.GetDisplayName` Target))))