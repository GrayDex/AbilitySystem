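; Gameplay ability for a character's melee attack, with combo-scaled damage and knockback.
; On activation it commits, has the owning BP_Character determine its combo, and plays that character's melee montage.
; A wait for the melee deal-damage gameplay event applies the damage effect to the event's target at the combo level, then pushes it away from the attacker with a brief stun.
; The ability ends whenever the montage completes, blends out or is interrupted or cancelled.
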(event `self.K2_ActivateAbility`
  ;[1 1 1] need calls for test cooldown ended setted in this in gameplayeffects
  (`self.K2_CommitAbility`)
  (bind _asbp_character (cast `/Game/Blueprints/Characters/BP_Character` (`self.GetOwningActorFromActorInfo`)))
  (`/Game/Blueprints/Characters/BP_Character.DetermineCombo` _asbp_character)
  (`AbilityTask_PlayMontageAndWait.CreatePlayMontageAndWaitProxy` "None" (`/Game/Blueprints/Characters/BP_Character.MeleeMontage` _asbp_character) 1.0 "None"
    (:`then`
      ;[1 1 1] wait event with any tag to continue execution. in event will be set target, that be set to apply damage in here
      (bind (_asynctaskproxy _payload) (`AbilityTask_WaitGameplayEvent.WaitGameplayEvent` (struct :`TagName` "skill.melee.dealDamage") null)
        (:`EventReceived`
          (bind (_eventtag _instigator _target) (break `GameplayEventData` _payload))
          ;[1 1 1] Call GE_AttackDamage for apply damage to target
          (`self.BP_ApplyGameplayEffectToTarget` (`AbilitySystemBlueprintLibrary.AbilityTargetDataFromActor` _target) "/Game/Blueprints/Characters/GameplayAbilities/A1_MeleeAttack/GE_MeleeAttack_Damage.GE_MeleeAttack_Damage_C" (`/Game/Blueprints/Characters/BP_Character.GEL_ComboDamage` _asbp_character))
          (bind _asbp_character_2 (cast `/Game/Blueprints/Characters/BP_Character` _target))
          (`/Game/Blueprints/Characters/BP_Character.PushCharacter` _asbp_character_2 (`KismetMathLibrary.Normal` (- (`Actor.K2_GetActorLocation` _asbp_character_2) (`Actor.K2_GetActorLocation` (`self.GetOwningActorFromActorInfo`)))) 200.0 0.1))))
    (:`OnCompleted`
      ;[1 1 1] Call event OnEndAbility
      (`self.K2_EndAbility` :!label _label))
    (:`OnBlendOut`
      (goto _label))
    (:`OnInterrupted`
      (goto _label))
    (:`OnCancelled`
      (goto _label))))

(event `self.K2_OnEndAbility`
  (params (bWasCancelled :type Boolean)))

(fn `Print`
  (params (Instigator :type "Object Object Reference") (Target :type "Actor Object Reference"))
  (`KismetSystemLibrary.PrintString` (`KismetStringLibrary.Concat_StrStr` "Instigator: " (`KismetSystemLibrary.GetDisplayName` Instigator)))
  (`KismetSystemLibrary.PrintString` (`KismetStringLibrary.Concat_StrStr` "Target: " (`KismetSystemLibrary.GetDisplayName` Target))))