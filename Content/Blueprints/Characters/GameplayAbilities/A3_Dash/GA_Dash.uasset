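; Dash gameplay ability that launches the owning BP_Character along its control rotation and damages, pushes and stuns characters it hits.
; Activation commits, triggers the UI cooldown, zeroes ground friction, applies a velocity-change impulse and sets pawn collision to Overlap while a montage plays.
; Damage gameplay events apply the damage effect and shove targets away from the owner.
; Montage end or interruption restores friction, switches pawn collision to Ignore and ends the ability.
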(event `self.K2_ActivateAbility`
  (`self.K2_CommitAbility`)
  (`self.DoUI_Colldown`)
  (bind _asbp_character (cast `/Game/Blueprints/Characters/BP_Character` (`self.GetOwningActorFromActorInfo`))
    (:`then`
      (bind _charactermovement (`Character.CharacterMovement` _asbp_character))
      (set `self.OriginalGroundFriction` (`CharacterMovementComponent.GroundFriction` _charactermovement))
      (set `CharacterMovementComponent.GroundFriction` 0.0 _charactermovement)
      (bind (_returnvalue_roll _returnvalue_pitch _returnvalue_yaw) (`KismetMathLibrary.BreakRotator` (`Pawn.GetControlRotation` _asbp_character)))
      ;[1 1 1] Custom
      (`Actor.K2_SetActorRotation` _asbp_character (`KismetMathLibrary.MakeRotator` 0.0 0.0 _returnvalue_yaw) false)
      (`CharacterMovementComponent.AddImpulse` _charactermovement (* (`KismetMathLibrary.GetForwardVector` (`KismetMathLibrary.MakeRotator` _returnvalue_roll _returnvalue_pitch _returnvalue_yaw)) 1500.0) true)
      (bind _playercharacter (`self.GetPlayerPawnAndController`))
      (`/Game/Blueprints/Characters/BP_Character.SetCollisionToPawn` _playercharacter "ECR_Overlap")
      (`AbilityTask_PlayMontageAndWait.CreatePlayMontageAndWaitProxy` "None" "/Game/Blueprints/Characters/Animations/AM_DashShinbi.AM_DashShinbi"
        (:`then`
          (bind (_asynctaskproxy _payload) (`AbilityTask_WaitGameplayEvent.WaitGameplayEvent` (struct :`TagName` "skill.dash.dealDamage") null)
            (:`EventReceived`
              (bind (_eventtag _instigator _target) (break `GameplayEventData` _payload))
              (`self.BP_ApplyGameplayEffectToTarget` (`AbilitySystemBlueprintLibrary.AbilityTargetDataFromActor` _target) "/Game/Blueprints/Characters/GameplayAbilities/A3_Dash/GE_Dash_Damage.GE_Dash_Damage_C")
              (bind _asbp_character_2 (cast `/Game/Blueprints/Characters/BP_Character` _target)
                (:`then`
                  (`/Game/Blueprints/Characters/BP_Character.PushCharacter` _asbp_character_2 (`KismetMathLibrary.Normal` (- (`Actor.K2_GetActorLocation` _asbp_character_2) (`Actor.K2_GetActorLocation` (`self.GetOwningActorFromActorInfo`)))) 1000.0 5.0))
                (:`CastFailed`
                  (`self.K2_EndAbility`))))))
        (:`OnCompleted`
          (set `CharacterMovementComponent.GroundFriction` (`self.OriginalGroundFriction`) _charactermovement :!label _label)
          (bind _playercharacter_2 (`self.GetPlayerPawnAndController`))
          (`/Game/Blueprints/Characters/BP_Character.SetCollisionToPawn` _playercharacter_2 "ECR_Ignore")
          (`self.K2_EndAbility`))
        (:`OnBlendOut`
          (goto _label))
        (:`OnInterrupted`
          (goto _label))
        (:`OnCancelled`
          (goto _label))))
    (:`CastFailed`
      (`self.K2_EndAbility`))))

(event `self.K2_OnEndAbility`
  (params (bWasCancelled :type Boolean))
  (`KismetSystemLibrary.PrintString` (`KismetStringLibrary.Concat_StrStr` (`KismetSystemLibrary.GetDisplayName` (`self.GetOwningActorFromActorInfo`)) "  Ability: " (`KismetSystemLibrary.GetObjectName` self) " end.")))