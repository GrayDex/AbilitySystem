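; Gameplay ability that casts a fireball for the player character.
; On activation it commits, triggers the UI cooldown and plays a Shinbi melee combo montage.
; When the montage completes or blends out, it spawns BP_FireBall at the character's actor transform, passing a GE_Burning effect spec, then ends.
; Interruption or cancellation ends the ability without spawning the projectile.
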(event `self.K2_ActivateAbility`
  (`self.K2_CommitAbility`)
  (`self.DoUI_Colldown`)
  (`AbilityTask_PlayMontageAndWait.CreatePlayMontageAndWaitProxy` "None" "/Game/Blueprints/Characters/Animations/AM_MeleeCombo01_Shinbi.AM_MeleeCombo01_Shinbi"
    (:`OnCompleted`
      (bind _playercharacter (`self.GetPlayerPawnAndController` :!label _label))
      (`|SpawnActorFromClass` "/Game/Blueprints/Characters/GameplayAbilities/FireBall/BP_FireBall.BP_FireBall_C" (`Actor.GetTransform` _playercharacter) "Undefined" "OverrideRootScale" _playercharacter (`self.MakeOutgoingGameplayEffectSpec` "/Game/Blueprints/Characters/GameplayAbilities/_General/GE_Burning.GE_Burning_C") _playercharacter)
      (`self.K2_EndAbility`))
    (:`OnBlendOut`
      (goto _label))
    (:`OnInterrupted`
      (`self.K2_EndAbility` :!label _label_2))
    (:`OnCancelled`
      (goto _label_2))))