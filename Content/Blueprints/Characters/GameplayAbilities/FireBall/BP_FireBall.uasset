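; BP_FireBall is the fireball actor for the character gameplay abilities, applying a gameplay effect to a hostile character it touches.
; Its sphere overlap casts both the other actor and the instigator to BP_Character, then asks the instigator whether the other is hostile.
; On a hostile hit it applies the effect through target data built from that actor and destroys itself.
; A timer started on BeginPlay destroys it after a fixed lifetime.
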(event `self.ReceiveBeginPlay`
  (`KismetSystemLibrary.K2_SetTimerDelegate` (delegate `TimeToDie`) 6.0))

(event `TimeToDie`
  (`self.K2_DestroyActor`))

(event `self.Sphere.OnComponentBeginOverlap`
  (params (OverlappedComponent :type "PrimitiveComponent Object Reference") (OtherActor :type "Actor Object Reference") (OtherComp :type "PrimitiveComponent Object Reference") (OtherBodyIndex :type Integer) (bFromSweep :type Boolean) (SweepResult :type "HitResult Structure (by ref)"))
  (bind _asbp_character (cast `/Game/Blueprints/Characters/BP_Character` OtherActor))
  (bind _asbp_character_2 (cast `/Game/Blueprints/Characters/BP_Character` (`self.GetInstigator`)))
  (bind _returnvalue (`CharacterBase.IsOtherHostile` _asbp_character_2 _asbp_character))
  (if _returnvalue
    (`CharacterBase.Apply_GESH_To_TDH` _asbp_character (`self.GameplayEffect`) (`AbilitySystemBlueprintLibrary.AbilityTargetDataFromActor` OtherActor))
    (`self.K2_DestroyActor`)))

(fn `UserConstructionScript`)