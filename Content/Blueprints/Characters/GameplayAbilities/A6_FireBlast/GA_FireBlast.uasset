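; GA_FireBlast is a gameplay ability that pulls enemies around the owner in, then blasts them away with damage and a stun.
; Montage gameplay events time both phases.
; The pull event gathers instant radius target data, commits cost and cooldown, and reuses PushEnemiesAway with reversed direction.
; The push event applies the damage effect to those stored targets and knocks them back with a longer stun.
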(event `self.K2_ActivateAbility`
  ;[1 1 1] Comment
  (`AbilityTask_PlayMontageAndWait.CreatePlayMontageAndWaitProxy` "None" "/Game/Blueprints/Characters/Animations/AM_FireBlast.AM_FireBlast"
    (:`then`
      (`AbilityTask_WaitGameplayEvent.WaitGameplayEvent` (struct :`TagName` "skill.fireBlast.pull") null
        (:`EventReceived`
          (bind (_asynctaskproxy _data) (`AbilityTask_WaitTargetData.WaitTargetData` "None" "Instant" "/Script/AbilitySystem.GATActorAroundOwner" 500.0 (struct) (struct) null)
            (:`then`
              (`AbilityTask_WaitGameplayEvent.WaitGameplayEvent` (struct :`TagName` "skill.fireBlast.push") null
                (:`EventReceived`
                  (`self.BP_ApplyGameplayEffectToTarget` (`self.TargetData`) "/Game/Blueprints/Characters/GameplayAbilities/A6_FireBlast/GE_FireBlast_Damage.GE_FireBlast_Damage_C")
                  (`self.PushEnemiesAway` (`self.TargetData`) 1 1500.0 2.0))))
            (:`ValidData`
              (set `self.TargetData` _data)
              (`self.K2_CommitAbility`)
              (`self.DoUI_Colldown`)
              (`self.PushEnemiesAway` (`self.TargetData`) -1 1500.0 0.6))
            (:`Cancelled`
              (`self.K2_EndAbility`))))))
    (:`OnCompleted`
      (`self.K2_EndAbility` :!label _label))
    (:`OnBlendOut`
      (goto _label))
    (:`OnInterrupted`
      (goto _label))
    (:`OnCancelled`
      (goto _label))))

(event `self.K2_OnEndAbility`
  (params (bWasCancelled :type Boolean)))