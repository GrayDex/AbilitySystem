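; Gameplay ability that fires a sustained laser from the player character.
; On activation it commits, plays a montage and, after a short delay, spawns BP_Laser on a mesh socket and enables camera-controlled rotation.
; Laser damage events apply a damage effect and push targets away from the beam's end detector with a brief stun, or end the ability once cost runs out.
; Ending removes mana drain, destroys the laser, restores rotation and triggers UI cooldown.
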(event `self.K2_ActivateAbility`
  ;[1 1 1] Activate Ability
  (`self.K2_CommitAbility`)
  (`AbilityTask_PlayMontageAndWait.CreatePlayMontageAndWaitProxy` "None" "/Game/Blueprints/Characters/Animations/AM_Laser_Shinbi.AM_Laser_Shinbi" 1.0 "Start"
    (:`then`
      (`KismetSystemLibrary.Delay` 0.4)
      (bind _playercharacter (`self.GetPlayerPawnAndController`))
      (bind (_asynctaskproxy _spawnedactor) (`AbilityTask_SpawnActor.SpawnActor` (struct) "/Game/Blueprints/Characters/GameplayAbilities/A4_Laser/Assets/BP_Laser.BP_Laser_C" _playercharacter)
        (:`Success`
          (bind _output_get (set `self.LaserActor` _spawnedactor))
          (`Actor.K2_AttachToComponent` _output_get (`Character.Mesh` _playercharacter) "LaserSocket" "SnapToTarget" "SnapToTarget" "KeepRelative" true)
          (`/Game/Blueprints/Characters/BP_Character.MakeCameraControlRotation` _playercharacter true)
          (bind (_asynctaskproxy_2 _payload) (`AbilityTask_WaitGameplayEvent.WaitGameplayEvent` (struct :`TagName` "skill.laser.dealDamage") null)
            (:`EventReceived`
              (bind _can (`self.IsCostStillAvaliable`))
              (if _can
                (bind (_eventtag _instigator _target _optionalobject _optionalobject2 _contexthandle _instigatortags _targettags _eventmagnitude _targetdata) (break `GameplayEventData` _payload))
                ;;[1 1 1] ApplyDamage to FullMassive
                (`self.BP_ApplyGameplayEffectToTarget` _targetdata "/Game/Blueprints/Characters/GameplayAbilities/A4_Laser/GE_Laser_Damage.GE_Laser_Damage_C")
                (for _array_element (`AbilitySystemBlueprintLibrary.GetActorsFromTargetData` _targetdata)
                  (bind _asbp_character (cast `/Game/Blueprints/Characters/BP_Character` _array_element))
                  (`/Game/Blueprints/Characters/BP_Character.PushCharacter` _asbp_character (`KismetMathLibrary.Normal` (- (`Actor.K2_GetActorLocation` _asbp_character) (`SceneComponent.K2_GetComponentLocation` (`/Game/Blueprints/Characters/GameplayAbilities/A4_Laser/Assets/BP_Laser.LaserEndDetector` (cast `/Game/Blueprints/Characters/GameplayAbilities/A4_Laser/Assets/BP_Laser` (`self.LaserActor`) :!pure true))))) 300.0 0.1))
                (else
                  (`self.K2_EndAbility`))))))
        (:`DidNotSpawn`
          (`self.K2_EndAbility`))))))

(event `self.K2_OnEndAbility`
  (params (bWasCancelled :type Boolean))
  ;[1 1 1] EndAbility
  (`self.BP_RemoveGameplayEffectFromOwnerWithAssetTags` (struct :`GameplayTags` (struct :`(TagName` "skill.laser.drainMana"))))
  (`Actor.K2_DestroyActor` (`self.LaserActor`))
  (bind _playercharacter (`self.GetPlayerPawnAndController`))
  (`/Game/Blueprints/Characters/BP_Character.MakeCameraControlRotation` _playercharacter false)
  (`self.DoUI_Colldown`))