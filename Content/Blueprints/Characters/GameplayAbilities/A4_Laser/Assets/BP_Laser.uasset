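; Laser beam actor for the A4_Laser gameplay ability that reports hostile characters touching the beam's end detector.
; Each tick it offsets the laser mesh's end bone through AM_Laser so the beam length follows LaserEndDetector.
; Detector overlaps maintain a list of characters hostile to the instigator.
; A looping timer sends that list, even when empty, as target data to the instigator in a Skill.laser.dealDamage gameplay event.
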(event `self.ReceiveBeginPlay`
  ;[1 1 1] BeginPlay
  (set `self.BeamOriginalLenght` (`KismetMathLibrary.VSize` (- (`SceneComponent.GetSocketLocation` (`self.LaserMesh`) "end") (`self.K2_GetActorLocation`))))
  ;[1 1 1] DealDamageEvent
  (`KismetSystemLibrary.K2_SetTimerDelegate` (delegate `DealDamageEvent`) 0.3 true))

(event `DealDamageEvent`
  (bind _returnvalue (`self.GetInstigator`))
  (bind _overlappingactors (`self.OverlappingActors`))
  ;[1 1 1] DealDamageEvent
  (if (> (`KismetArrayLibrary.Array_Length` _overlappingactors) 0)
    _
    (else
      _))
  (`AbilitySystemBlueprintLibrary.SendGameplayEventToActor` _returnvalue (struct :`TagName` "skill.laser.dealDamage") (make `GameplayEventData` (struct) _returnvalue null null null (struct) (struct) (struct) 0.0 (`AbilitySystemBlueprintLibrary.AbilityTargetDataFromActorArray` _overlappingactors))))

(event `self.ReceiveTick`
  (params (DeltaSeconds :type "Float (single-precision)"))
  ;[1 1 1] Tick
  (bind _asam_laser (cast `/Game/Blueprints/Characters/GameplayAbilities/A4_Laser/Assets/AM_Laser` (`SkeletalMeshComponent.GetAnimInstance` (`self.LaserMesh`))))
  (set `/Game/Blueprints/Characters/GameplayAbilities/A4_Laser/Assets/AM_Laser.Offset_EndBone` (`KismetMathLibrary.MakeVector` (- (`KismetMathLibrary.VSize` (- (`SceneComponent.K2_GetComponentLocation` (`self.LaserEndDetector`)) (`self.K2_GetActorLocation`))) (`self.BeamOriginalLenght`))) _asam_laser))

(event `self.LaserEndDetector.OnComponentBeginOverlap`
  (params (OverlappedComponent :type "PrimitiveComponent Object Reference") (OtherActor :type "Actor Object Reference") (OtherComp :type "PrimitiveComponent Object Reference") (OtherBodyIndex :type Integer) (bFromSweep :type Boolean) (SweepResult :type "HitResult Structure (by ref)"))
  ;[1 1 1] LaserEndDetector OnBeginOverlap
  (bind _asbp_character (cast `/Game/Blueprints/Characters/BP_Character` OtherActor))
  (bind _asbp_character_2 (cast `/Game/Blueprints/Characters/BP_Character` (`self.GetInstigator`)))
  (bind _returnvalue (`CharacterBase.IsOtherHostile` _asbp_character_2 _asbp_character))
  (if _returnvalue
    (`KismetArrayLibrary.Array_AddUnique` (`self.OverlappingActors`) _asbp_character)))

(event `self.LaserEndDetector.OnComponentEndOverlap`
  (params (OverlappedComponent :type "PrimitiveComponent Object Reference") (OtherActor :type "Actor Object Reference") (OtherComp :type "PrimitiveComponent Object Reference") (OtherBodyIndex :type Integer))
  ;[1 1 1] LaserEndDetector OnEndOverlap
  (bind _asbp_character (cast `/Game/Blueprints/Characters/BP_Character` OtherActor))
  (`KismetArrayLibrary.Array_RemoveItem` (`self.OverlappingActors`) _asbp_character))

(fn `UserConstructionScript`)