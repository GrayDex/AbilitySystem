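; GA_Base is a base Gameplay Ability that provides shared helpers for player abilities.
; GetPlayerPawnAndController casts the owning actor to BP_Character and its controller to BP_PlayerController.
; DoUIColldown uses that controller to loop through the primary UI's ability slots and start the cooldown on those whose ability class matches this ability's info.
; It has no activation or end logic of its own.
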(fn `DoUI_Colldown`
  (bind (_playercharacter _playercontroller) (`self.GetPlayerPawnAndController`))
  (`/Engine/EditorBlueprintResources/StandardMacros.IsValid` _playercontroller
    (:`Is Valid`
      (for _array_element (`/Game/Blueprints/UI/Player_PrimaryUI/WBP_PrimaryUI.AbilitySlots` (`/Game/Blueprints/BP_PlayerController.PrimaryUI` _playercontroller))
        (bind _returnvalue (`self.GetAbilityInfo`))
        (bind (_abilityinfo_cooldownduration _abilityinfo_cost _abilityinfo_costtype _abilityinfo_uimat _abilityinfo_abilityclass) (break `GameplayAbilityInfo` (`/Game/Blueprints/UI/Player_PrimaryUI/AbilitySlotComponent/WBP_AbilitySlot.AbilityInfo` _array_element)))
        (if (== (`.AbilityClass` (break `GameplayAbilityInfo` _returnvalue)) _abilityinfo_abilityclass)
          (`/Game/Blueprints/UI/Player_PrimaryUI/AbilitySlotComponent/WBP_AbilitySlot.StartCooldown` _array_element))))))

(fn `GetPlayerPawnAndController`
  (returns (PlayerCharacter :type "/Game/Blueprints/Characters/BP_Character Object Reference") (PlayerController :type "/Game/Blueprints/BP_PlayerController Object Reference"))
  (bind _asbp_character (cast `/Game/Blueprints/Characters/BP_Character` (`self.GetOwningActorFromActorInfo`)))
  (bind _asbp_player_controller (cast `/Game/Blueprints/BP_PlayerController` (`Pawn.GetController` _asbp_character))
    (:`then`
      _)
    (:`CastFailed`
      _))
  (return _asbp_character _asbp_player_controller))