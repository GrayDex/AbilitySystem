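; Gameplay ability for a targeted ground blast that damages characters, launches them upward and stuns them.
; After a targeting montage, it waits for user-confirmed target data from GATActor_GroundBlast; cancelling ends the ability.
; Confirmation commits the ability, starts the UI cooldown, turns the player to control yaw and plays the cast montage.
; As the cast starts, that target data drives the damage effect, blast particle location and character pushes.
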(event `self.K2_ActivateAbility`
  ;[1 1 1] Activate ability
  (`AbilityTask_PlayMontageAndWait.CreatePlayMontageAndWaitProxy` "None" "/Game/Blueprints/Characters/Animations/AM_GroundBlastTargeting_Shinbi.AM_GroundBlastTargeting_Shinbi"
    (:`then`
      (`KismetSystemLibrary.Delay` (`AnimSequenceBase.SequenceLength` (`self.GetCurrentMontage`)))
      (bind (_asynctaskproxy _data) (`AbilityTask_WaitTargetData.WaitTargetData` "None" "UserConfirmed" "/Game/Blueprints/Characters/GameplayAbilities/A5_GroundBlast/GATActor_GroundBlast.GATActor_GroundBlast_C" 200.0 (struct) (struct) null)
        (:`ValidData`
          (bind (_playercharacter _playercontroller) (`self.GetPlayerPawnAndController`))
          (set `/Game/Blueprints/BP_PlayerController.Targeting` false _playercontroller)
          (`self.K2_CommitAbility`)
          (`self.DoUI_Colldown`)
          (bind (_playercharacter_2 _playercontroller_2) (`self.GetPlayerPawnAndController`))
          (bind (_returnvalue_roll _returnvalue_pitch _returnvalue_yaw) (`KismetMathLibrary.BreakRotator` (`Controller.GetControlRotation` _playercontroller_2)))
          (`Actor.K2_SetActorRotation` _playercharacter_2 (`KismetMathLibrary.MakeRotator` 0.0 0.0 _returnvalue_yaw) false)
          (`AbilityTask_PlayMontageAndWait.CreatePlayMontageAndWaitProxy` "None" "/Game/Blueprints/Characters/Animations/AM_GroundBlast_Cast_Shinbi.AM_GroundBlast_Cast_Shinbi" 2.0
            (:`then`
              (`self.BP_ApplyGameplayEffectToTarget` _data "/Game/Blueprints/Characters/GameplayAbilities/A5_GroundBlast/GE_GroundBlast_Damage.GE_GroundBlast_Damage_C")
              (`GameplayStatics.SpawnEmitterAtLocation` "/Game/Blueprints/Characters/GameplayAbilities/A5_GroundBlast/Assets/P_GroundBlast.P_GroundBlast" (`AbilitySystemBlueprintLibrary.GetTargetDataEndPoint` _data (- (`AbilitySystemBlueprintLibrary.GetDataCountFromTargetData` _data) 1)) (struct))
              (for _array_element (`AbilitySystemBlueprintLibrary.GetActorsFromTargetData` _data)
                (bind _asbp_character (cast `/Game/Blueprints/Characters/BP_Character` _array_element))
                (`/Game/Blueprints/Characters/BP_Character.PushCharacter` _asbp_character (0.0 0.0 1.0) 400.0 2.0)))
            (:`OnCompleted`
              (`self.K2_EndAbility` :!label _label))
            (:`OnBlendOut`
              (goto _label))
            (:`OnInterrupted`
              (goto _label))
            (:`OnCancelled`
              (goto _label))))
        (:`Cancelled`
          (`self.K2_EndAbility`))))))

(event `self.K2_OnEndAbility`
  (params (bWasCancelled :type Boolean)))