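; Base Gameplay Ability that supplies shared helper functions and has no activation logic of its own.
; It resolves the owning player character and controller, then uses them to start cooldowns on matching UI ability slots.
; A cost check compares the ability's negated cost against current Health, Mana or Strenght.
; A push helper shoves targeted characters along the owner-to-target vector, scaled by Direction, with strength and stun duration.
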(fn `DoUI_Colldown`
  (bind (_playercharacter _playercontroller) (`self.GetPlayerPawnAndController`))
  (`/Engine/EditorBlueprintResources/StandardMacros.IsValid` _playercontroller
    (:`Is Valid`
      (for _array_element (`/Game/Blueprints/UI/Player_PrimaryUI/WBP_PrimaryUI.AbilitySlots` (`/Game/Blueprints/BP_PlayerController.PrimaryUI` _playercontroller))
        (bind _returnvalue (`self.GetAbilityInfo`))
        (bind (_abilityinfo_cooldownduration _abilityinfo_cost _abilityinfo_costtype _abilityinfo_uimat _abilityinfo_abilityclass) (break `GameplayAbilityInfo` (`/Game/Blueprints/UI/Player_PrimaryUI/AbilitySlotComponent/WBP_AbilitySlot.AbilityInfo` _array_element)))
        (if (== (`.AbilityClass` (break `GameplayAbilityInfo` _returnvalue)) _abilityinfo_abilityclass)
          (`/Game/Blueprints/UI/Player_PrimaryUI/AbilitySlotComponent/WBP_AbilitySlot.StartCooldown` _array_element))))))

(fn `GetNormalVectorToTarget`
  (params (Target :type "Actor Object Reference"))
  (returns (Success :type Boolean) (TargetCharacter :type "/Game/Blueprints/Characters/BP_Character Object Reference") (NormalVector :type "Vector Structure"))
  (bind _asbp_character (cast `/Game/Blueprints/Characters/BP_Character` Target)
    (:`then`
      (return true _asbp_character (`KismetMathLibrary.Normal` (- (`Actor.K2_GetActorLocation` _asbp_character) (`Actor.K2_GetActorLocation` (`self.GetOwningActorFromActorInfo`))))))
    (:`CastFailed`
      (return false null (0.0 0.0 0.0)))))

(fn `GetPlayerPawnAndController`
  (returns (PlayerCharacter :type "/Game/Blueprints/Characters/BP_Character Object Reference") (PlayerController :type "/Game/Blueprints/BP_PlayerController Object Reference"))
  (bind _asbp_character (cast `/Game/Blueprints/Characters/BP_Character` (`self.GetOwningActorFromActorInfo`)))
  (bind _asbp_player_controller (cast `/Game/Blueprints/BP_PlayerController` (`Pawn.GetController` _asbp_character))
    (:`then`
      _)
    (:`CastFailed`
      _))
  (return _asbp_character _asbp_player_controller))

(fn `IsCostStillAvaliable`
  (returns (Can :type Boolean))
  (locals (Cost :type "Float (double-precision)"))
  (bind _cost (`local.Cost`))
  (bind _returnvalue (`self.GetAbilityInfo`))
  (set `local.Cost` (* -1 (`.Cost` (break `GameplayAbilityInfo` _returnvalue))))
  (switch `EAbilityCostType` (`.CostType` (break `GameplayAbilityInfo` _returnvalue))
    (:`Health`
      (bind _playercharacter (`self.GetPlayerPawnAndController`))
      (bind (_health_basevalue _health_currentvalue) (break `GameplayAttributeData` (`AttributeSetBase.Health` (`CharacterBase.AttributeSetBaseComp` _playercharacter))))
      (return (>= _health_currentvalue _cost)))
    (:`Mana`
      (bind _playercharacter_2 (`self.GetPlayerPawnAndController`))
      (bind (_mana_basevalue _mana_currentvalue) (break `GameplayAttributeData` (`AttributeSetBase.Mana` (`CharacterBase.AttributeSetBaseComp` _playercharacter_2))))
      (return (>= _mana_currentvalue _cost)))
    (:`Strenght`
      (bind _playercharacter_3 (`self.GetPlayerPawnAndController`))
      (bind (_strenght_basevalue _strenght_currentvalue) (break `GameplayAttributeData` (`AttributeSetBase.Strenght` (`CharacterBase.AttributeSetBaseComp` _playercharacter_3))))
      (return (>= _strenght_currentvalue _cost)))))

(fn `PushEnemiesAway`
  (params (TargetData :type "GameplayAbilityTargetDataHandle Structure (by ref)") (Direction :type Integer :default 1) (PushStrenght :type "Float (double-precision)") (StunDuration :type "Float (double-precision)"))
  (for _array_element (`AbilitySystemBlueprintLibrary.GetActorsFromTargetData` TargetData)
    (bind (_success _targetcharacter _normalvector) (`self.GetNormalVectorToTarget` _array_element))
    (if _success
      (`/Game/Blueprints/Characters/BP_Character.PushCharacter` _targetcharacter (* _normalvector Direction) PushStrenght StunDuration)))
  (return))