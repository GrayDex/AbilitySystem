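; Gameplay Ability that lets a character cast health regeneration on itself.
; It plays the Shinbi regen cast montage, and Completed or Blend Out commits the ability, triggers the UI cooldown, applies the regeneration GameplayEffect to the owner and ends.
; The commit happens only after the cast, with its result unchecked, so interruption or cancellation ends the ability without committing.
; Ending prints a debug message.
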(event `self.K2_ActivateAbility`
  (`AbilityTask_PlayMontageAndWait.CreatePlayMontageAndWaitProxy` "None" "/Game/Blueprints/Characters/Animations/AM_RegenCast_Shinbi.AM_RegenCast_Shinbi"
    (:`OnCompleted`
      ;[0.2344 0.1218 1] This CommitAbility run calculation ability attributes: cooldown etc.
      (`self.K2_CommitAbility` :!label _label)
      (`self.DoUI_Colldown`)
      (`self.BP_ApplyGameplayEffectToOwner` "/Game/Blueprints/Characters/GameplayAbilities/A2_HealthRegen/GE_HealthRegen_Regeneration.GE_HealthRegen_Regeneration_C")
      (`self.K2_EndAbility`))
    (:`OnBlendOut`
      (goto _label))
    (:`OnInterrupted`
      (`self.K2_EndAbility` :!label _label_2))
    (:`OnCancelled`
      (goto _label_2))))

(event `self.K2_OnEndAbility`
  (params (bWasCancelled :type Boolean))
  (`KismetSystemLibrary.PrintString` (`KismetStringLibrary.Concat_StrStr` "Ability: " (`KismetSystemLibrary.GetObjectName` self) " end.")))