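; BP_Character is a character Blueprint for Gameplay Ability System combat, with melee, dash hit detection, knockback and death.
; It acquires initial abilities on BeginPlay and activates GA_MeleeAttack for melee.
; Sword and capsule overlaps with hostile characters send melee and dash damage gameplay events to itself, the capsule skipping excluded characters.
; PushCharacter briefly zeroes ground friction for an impulse with optional stun; Die plays a montage, then destroys the actor.
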(event `self.ReceiveBeginPlay`
  ;[1 1 1] BeginPlay
  ;;[1 1 1] Create abilities
  (`self.AcquareAbilities` (`self.InitialAbilities`)))

(event `MileeAttack`
  ;[1 1 1] Binding GA_MeleeAttack
  (`AbilitySystemComponent.TryActivateAbilityByClass` (`self.AbilitySystemComp`) "/Game/Blueprints/Characters/GameplayAbilities/A1_MeleeAttack/GA_MeleeAttack.GA_MeleeAttack_C" true))

(event `self.BP_Die`
  ;[1 1 1] Die event
  (`self.PlayAnimMontage` "/Game/Blueprints/Characters/Animations/AM_Die_Shinbi.AM_Die_Shinbi" 1.0 "None")
  (`KismetSystemLibrary.Delay` 2.0)
  (`self.K2_DestroyActor`))

(event `self.SwordCollider.OnComponentBeginOverlap`
  (params (OverlappedComponent :type "PrimitiveComponent Object Reference") (OtherActor :type "Actor Object Reference") (OtherComp :type "PrimitiveComponent Object Reference") (OtherBodyIndex :type Integer) (bFromSweep :type Boolean) (SweepResult :type "HitResult Structure (by ref)"))
  ;[1 1 1] SwordCollider event OnComponentBeginOverlap
  (if (!= OtherActor self)
    (bind (_isenemy _gameplayeventdata) (`self.IsEnemy` OtherActor))
    (if _isenemy
      (`AbilitySystemBlueprintLibrary.SendGameplayEventToActor` self (struct :`TagName` "skill.melee.dealDamage") _gameplayeventdata))))

(event `self.CapsuleComponent.OnComponentBeginOverlap`
  (params (OverlappedComponent :type "PrimitiveComponent Object Reference") (OtherActor :type "Actor Object Reference") (OtherComp :type "PrimitiveComponent Object Reference") (OtherBodyIndex :type Integer) (bFromSweep :type Boolean) (SweepResult :type "HitResult Structure (by ref)"))
  ;[1 1 1] CapsuleComponent event OnComponentBeginOverlap
  (bind (_isenemy _gameplayeventdata) (`self.IsEnemy` OtherActor))
  (if _isenemy
    (bind _asbp_character (cast `/Game/Blueprints/Characters/BP_Character` OtherActor))
    (if (not (`KismetArrayLibrary.Array_Contains` (`self.OverlapExclude`) _asbp_character))
      (`AbilitySystemBlueprintLibrary.SendGameplayEventToActor` self (struct :`TagName` "skill.dash.dealDamage") _gameplayeventdata))))

(event `PushCharacter`
  (params (ImpulseDirection :type "Vector Structure") (PushStrenght :type "Float (double-precision)") (StunDuration :type "Float (double-precision)"))
  (bind _charactermovement (`self.CharacterMovement`))
  ;[1 1 1] Push this character
  (set `self.DefaultGroundFriction` (`CharacterMovementComponent.GroundFriction` _charactermovement))
  (set `CharacterMovementComponent.GroundFriction` 0.0 _charactermovement)
  (`CharacterMovementComponent.AddImpulse` _charactermovement (* ImpulseDirection PushStrenght) true)
  (if (> StunDuration 0.0)
    (`self.HitStun` StunDuration))
  (`KismetSystemLibrary.Delay` 0.3)
  (set `CharacterMovementComponent.GroundFriction` (`self.DefaultGroundFriction`) (`self.CharacterMovement`)))

(fn `IsEnemy`
  (params (OtherActor :type "Actor Object Reference"))
  (returns (IsEnemy :type Boolean) (GameplayEventData :type "GameplayEventData Structure"))
  (bind _asbp_character (cast `/Game/Blueprints/Characters/BP_Character` OtherActor)
    (:`then`
      (bind _returnvalue (`self.IsOtherHostile` _asbp_character))
      (if _returnvalue
        (return true (make `GameplayEventData` (struct) self OtherActor))
        (else
          _)))
    (:`CastFailed`
      _))
  (return false))

(fn `SetCollisionToPawn`
  (params (NewResponse :type "ECollisionResponse Enum" :default "ECR_Ignore"))
  (`PrimitiveComponent.SetCollisionResponseToChannel` (`self.CapsuleComponent`) "ECC_Pawn" NewResponse))

(fn `UserConstructionScript`)